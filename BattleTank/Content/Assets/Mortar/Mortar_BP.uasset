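; Mortar Blueprint that reuses the tank aiming component and health bar for a mortar with a dome turret and barrel.
; On BeginPlay it initialises TankAiming with the Dome as turret and the Barrel as barrel.
; It then casts the HealthBarComponent's widget to HealthBar and sets itself as that widget's TankRef.
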(event `self.ReceiveBeginPlay`
  (`TankAimingComponent.initialise` (`self.TankAiming`) (`self.Dome`) (`self.Barrel`))
  (`self.initialiseHealthBar`))

(fn `initialiseHealthBar`
  (bind _ashealth_bar (cast `/Game/UI/HealthBar` (`WidgetComponent.GetUserWidgetObject` (`self.HealthBarComponent`))))
  (set `/Game/UI/HealthBar.tankRef` self _ashealth_bar))

(fn `UserConstructionScript`)