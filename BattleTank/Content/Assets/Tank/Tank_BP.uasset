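; Tank pawn Blueprint that wires player input to movement, aiming, firing and an orbiting camera.
; On BeginPlay it hands turret and barrel to TankAiming, both tracks to TankMovement, and itself to the HealthBar widget.
; Move and fire inputs forward to those components, while aim axes yaw the AzimuthGimbal and pitch the SpringArm within clamped elevation limits.
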(event `self.ReceiveBeginPlay`
  (`TankAimingComponent.initialise` (`self.TankAiming`) (`self.Turret`) (`self.Barrel`))
  (`TankMovementComponent.initialise` (`self.TankMovement`) (`self.LeftTrack`) (`self.RightTrack`))
  (`self.initialiseHealthBar`))

(event `self.ReceiveTick`
  (params (DeltaSeconds :type "Float (single-precision)")))

(event `InputAxis|AimAzimuth`
  (params (AxisValue :type "Float (single-precision)"))
  ;[1 1 1] Camera Input Binding
  (`SceneComponent.K2_AddLocalRotation` (`self.AzimuthGimbal`) (`KismetMathLibrary.MakeRotator` 0.0 0.0 AxisValue) false false))

(event `InputAxis|MoveForward`
  (params (AxisValue :type "Float (single-precision)"))
  ;[1 1 1] Movement Input Binding
  (`TankMovementComponent.intendMoveForward` (`self.TankMovement`) AxisValue))

(event `InputAxis|MoveRight`
  (params (AxisValue :type "Float (single-precision)"))
  ;[1 1 1] Movement Input Binding
  (`TankMovementComponent.intendTurnRight` (`self.TankMovement`) AxisValue))

(event `InputAxis|AimElevation`
  (params (AxisValue :type "Float (single-precision)"))
  ;[1 1 1] Camera Input Binding
  (`SceneComponent.K2_SetRelativeRotation` (`self.SpringArm`) (`KismetMathLibrary.MakeRotator` 0.0 (`KismetMathLibrary.FClamp` (+ AxisValue (.pitch (`SceneComponent.RelativeRotation` (`self.SpringArm`)))) (`self.minCameraElevation`) (`self.maxCameraElevation`))) false false))

(event `InputAction|Fire`
  (params (Key :type "Key Structure"))
  ;[1 1 1] Action Bindings
  (:`Pressed`
    (`TankAimingComponent.fire` (`self.TankAiming`))))

(fn `initialiseHealthBar`
  (bind _ashealth_bar (cast `/Game/UI/HealthBar` (`WidgetComponent.GetUserWidgetObject` (`self.HealthBarComponent`))))
  (set `/Game/UI/HealthBar.tankRef` self _ashealth_bar))

(fn `UserConstructionScript`)